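; Homing missile projectile that seeks the first player's pawn and explodes when its box overlaps any actor other than its owner.
; On BeginPlay it targets a scene component on that pawn, draws a debug sphere there, and a timeline scales homing acceleration.
; Homing switches off two seconds after the timeline ends, so the missile stops tracking.
; Explode passes radius damage, sound, particles and camera shake to StartExplosion, then destroys the missile.
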(event OnComponentBeginOverlap(Box)
  (params (OverlappedComponent :type Primitive%20Component%20Object%20Reference) (OtherActor :type Actor%20Object%20Reference) (OtherComp :type Primitive%20Component%20Object%20Reference) (OtherBodyIndex :type Integer) (bFromSweep :type Boolean) (SweepResult :type Hit%20Result%20Structure%20%28by%20ref%29))
  (if (not (== OtherActor (Components|GetOwner)))
    (CallFunction|Explode)))

(event Custom|Explode
  (Class|PerformExplosion|StartExplosion 0.1 (Transformation|GetActorLocation) 3e+02 self 0 "/Game/MilitaryWeapDark/Sound/RocketLauncher/RocketLauncher_Explosion_Cue.RocketLauncher_Explosion_Cue" "/Game/MilitaryWeapDark/FX/P_Grenade_Explosion_01.P_Grenade_Explosion_01" "/Game/Blueprints/Damage/ExplosionDamage.ExplosionDamage_C" "/Game/Blueprints/Camera/CameraShake/ExplosionCameraShake.ExplosionCameraShake_C" 4.0)
  (Components|DestroyComponent (Variables|Default|GetRocketLauncher_InAirLoop_Cue))
  (Actor|DestroyActor))

(event EventBeginPlay
  (bind _projectilemovement (Variables|Default|GetProjectileMovement))
  (bind _projectilemovement_2 (Variables|Default|GetProjectileMovement))
  (bind _output_get (Variables|/Script/Engine.ProjectileMovementComponent|SetHomingTargetComponent _projectilemovement_2 (Actor|GetComponentbyClass (Game|Player|GetPlayerPawn 0) "/Script/Engine.SceneComponent")))
  (Variables|/Script/Engine.ProjectileMovementComponent|SetbIsHomingProjectile _projectilemovement_2 true)
  (Rendering|Debug|DrawDebugSphere (Transformation|GetWorldLocation _output_get) 2e+01 12 "(R=1.000000,G=1.000000,B=1.000000,A=1.000000)" 4.0)
  (bind _newtrack_0 (Timeline|Timeline_0 PlayFromStart)
    (:Update
      (Variables|/Script/Engine.ProjectileMovementComponent|SetHomingAccelerationMagnitude _projectilemovement (* 10000 _newtrack_0)))
    (:Finished
      (Utilities|FlowControl|Delay 2.0)
      (Variables|/Script/Engine.ProjectileMovementComponent|SetbIsHomingProjectile _projectilemovement false))))

(event EventTick
  (params (DeltaSeconds :type Float%20%28single-precision%29)))

(fn ConstructionScript)