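; Wanted-level manager for a police response to player violence, though only its BeginPlay setup is live.
; BeginPlay caches TargetPoints as spawn points and creates the WBP_WantedLevel HUD widget bound to itself.
; Events and functions are empty stubs.
; Disconnected graphs hold the unused logic: data-table violence scoring with falloff, staggered police spawns, timed backup under AI caps, and cooldown.
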(event Custom|StartAction)

(event Custom|CallForPolice)

(event Custom|CallForBackup)

(event Custom|SpawnPolice
  (params (PoliceType%20Num :type Integer)))

(event Custom|RegisterViolence
  (params (NewParam :type EViolenceType%20Enum :default "EVT_None")))

(event EventBeginPlay
  (bind _outactors (Actor|GetAllActorsOfClass "/Script/Engine.TargetPoint"))
  (Variables|Default|SetEnemySpawnPoint _outactors)
  (Variables|Default|SetTargetPoints _outactors)
  (bind _returnvalue (UserInterface|CreateWidget "/Game/Blueprints/WantedSystem/WBP_WantedLevel.WBP_WantedLevel_C"))
  (UserInterface|Viewport|AddtoViewport _returnvalue 0)
  (Default|SetObject _returnvalue self))

(fn ConstructionScript)

(fn DecreaseViolence)

(fn DecreaseViolenceOvertime)

(fn AIDead)