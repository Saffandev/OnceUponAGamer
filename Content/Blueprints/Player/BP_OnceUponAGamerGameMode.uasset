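; Game mode that starts the player and handles checkpoint save and restore through BP_SaveGame.
; On player start it async-loads any existing save to restore position, streamed level, weapons, throwables and health/shield, otherwise streams the first area and creates a save object.
; A fade widget covers startup before the HUD appears.
; SaveTheGame shows a brief saving notice and async-saves player state with the CheckPoint's level and location; Quit is an empty stub.
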(event Custom|Quit
  (params (bIsQuit :type Boolean))
  ;[1 1 1] Save Data
)

(event Custom|SaveTheGame
  (bind _savegame (Variables|Default|GetSaveGame))
  (bind _checkpoint (Variables|Default|GetCheckPoint))
  ;[1 1 1] Save Data
  (Variables|Default|SetbisCheckpointSave true)
  (Variables|Default|GetSaveGame
    (:then
      (Variables|Default|GetPlayerCharacter
        (:then
          (Utilities|FlowControl|Sequence
            (:then_0
              (bind _returnvalue (UserInterface|CreateWidget "/Game/Blueprints/Widget/WBP_SavingText.WBP_SavingText_C"))
              (UserInterface|Viewport|AddtoViewport _returnvalue 0)
              (Utilities|FlowControl|Delay 2.0)
              (Widget|RemovefromParent _returnvalue))
            (:then_1
              (bind _returnvalue_2 (Class|PlayerCharacter|GetWeaponData (Variables|Default|GetPlayerCharacter) true))
              (Variables|/Game/Blueprints/BP_SaveGame.BP_SaveGame_C|SetSecondaryWeaponData (Variables|Default|GetSaveGame) _returnvalue_2)
              (bind _returnvalue_3 (Class|PlayerCharacter|GetWeaponData (Variables|Default|GetPlayerCharacter) false))
              (Variables|/Game/Blueprints/BP_SaveGame.BP_SaveGame_C|SetPrimaryWeaponData (Variables|Default|GetSaveGame) _returnvalue_3))
            (:then_2
              (Variables|/Game/Blueprints/BP_SaveGame.BP_SaveGame_C|SetPlayerHealth (Variables|Default|GetSaveGame) (Variables|/Script/OnceUponAGamer.PlayerCharacter|GetCurrentHealth (Variables|Default|GetPlayerCharacter)))
              (Variables|/Game/Blueprints/BP_SaveGame.BP_SaveGame_C|SetPlayerShield (Variables|Default|GetSaveGame) (Variables|/Script/OnceUponAGamer.PlayerCharacter|GetCurrentShield (Variables|Default|GetPlayerCharacter))))
            (:then_3
              (bind _returnvalue_4 (Class|PlayerCharacter|GetThrowableData (Variables|Default|GetPlayerCharacter) false))
              (Variables|/Game/Blueprints/BP_SaveGame.BP_SaveGame_C|SetPrimaryThrowable (Variables|Default|GetSaveGame) _returnvalue_4)
              (bind _returnvalue_5 (Class|PlayerCharacter|GetThrowableData (Variables|Default|GetPlayerCharacter) true))
              (Variables|/Game/Blueprints/BP_SaveGame.BP_SaveGame_C|SetSecondaryThrowable (Variables|Default|GetSaveGame) _returnvalue_5)
              (Variables|/Game/Blueprints/BP_SaveGame.BP_SaveGame_C|SetLevelToLoad (Variables|Default|GetSaveGame) (Variables|/Game/Blueprints/Interactiables/BP_LevelCheckpoint.BP_LevelCheckpoint_C|GetLevelName _checkpoint))
              (Variables|/Game/Blueprints/BP_SaveGame.BP_SaveGame_C|SetPlayerSpawnLocation (Variables|Default|GetSaveGame) (Transformation|GetActorLocation _checkpoint)))
            (:then_4
              (|AsyncSaveGametoSlot (Variables|Default|GetSaveGame) (Variables|/Game/Blueprints/BP_SaveGame.BP_SaveGame_C|GetSaveGameSlot _savegame) (Variables|/Game/Blueprints/BP_SaveGame.BP_SaveGame_C|GetUserIndex _savegame)))))
        (:else)))
    (:else)))

(event EventBeginPlay)

(event EventTick
  (params (DeltaSeconds :type Float%20%28single-precision%29)))

(event EventHandleStartingNewPlayer
  (params (NewPlayer :type Player%20Controller%20Object%20Reference))
  (Class|GameModeBase|RestartPlayer NewPlayer)
  (Utilities|FlowControl|Sequence
    (:then_0
      (bind _asplayer_character (Utilities|Casting|CastToPlayerCharacter (Game|GetPlayerCharacter 0)))
      (Variables|Default|SetPlayerCharacter _asplayer_character)
      (bind _returnvalue (UserInterface|CreateWidget "/Game/Blueprints/Widget/WBP_FadeLevel.WBP_FadeLevel_C"))
      (bind _output_get (Variables|Default|SetWD_Fade _returnvalue))
      (UserInterface|Viewport|AddtoViewport _output_get 0)
      (Input|SetInputModeGameOnly (Game|GetPlayerController 0)))
    (:then_1
      ;[0 0 0] Load Save Data
      (bind _returnvalue_2 (SaveGame|DoesSaveGameExist "SaveGame"))
      (if _returnvalue_2
        (bind _savegame (|AsyncLoadGamefromSlot "SaveGame")
          (:Completed
            (bind _asbp_save_game (Utilities|Casting|CastToBP_SaveGame _savegame))
            (Variables|Default|SetSaveGame _asbp_save_game)
            (Transformation|SetActorLocation (Variables|Default|GetPlayerCharacter) (Variables|/Game/Blueprints/BP_SaveGame.BP_SaveGame_C|GetPlayerSpawnLocation (Variables|Default|GetSaveGame)) false false)
            (Game|LoadStreamLevel(byName) (Variables|/Game/Blueprints/BP_SaveGame.BP_SaveGame_C|GetLevelToLoad (Variables|Default|GetSaveGame)) true)
            (Utilities|FlowControl|Sequence
              (:then_0
                (Class|PlayerCharacter|SetWeaponData (Variables|Default|GetPlayerCharacter) true (Variables|/Game/Blueprints/BP_SaveGame.BP_SaveGame_C|GetSecondaryWeaponData (Variables|Default|GetSaveGame)))
                (Class|PlayerCharacter|SetWeaponData (Variables|Default|GetPlayerCharacter) false (Variables|/Game/Blueprints/BP_SaveGame.BP_SaveGame_C|GetPrimaryWeaponData (Variables|Default|GetSaveGame)))
                (Class|PlayerCharacter|SetHealthShield (Variables|Default|GetPlayerCharacter) (Variables|/Game/Blueprints/BP_SaveGame.BP_SaveGame_C|GetPlayerHealth (Variables|Default|GetSaveGame)) (Variables|/Game/Blueprints/BP_SaveGame.BP_SaveGame_C|GetPlayerShield (Variables|Default|GetSaveGame))))
              (:then_1
                (Class|PlayerCharacter|SetThrowableData (Variables|Default|GetPlayerCharacter) (Variables|/Game/Blueprints/BP_SaveGame.BP_SaveGame_C|GetPrimaryThrowable (Variables|Default|GetSaveGame)) false)
                (Class|PlayerCharacter|SetThrowableData (Variables|Default|GetPlayerCharacter) (Variables|/Game/Blueprints/BP_SaveGame.BP_SaveGame_C|GetSecondaryThrowable (Variables|Default|GetSaveGame)) true))
              (:then_3
                (UserInterface|Animation|PlayAnimation (Variables|Default|GetWD_Fade) (Variables|/Game/Blueprints/Widget/WBP_FadeLevel.WBP_FadeLevel_C|GetFade (Variables|Default|GetWD_Fade)) 0.0 1 "Forward" 1.0 false :!label _label)
                (bind _returnvalue_3 (UserInterface|CreateWidget "/Game/Blueprints/Widget/WBP_PlayerHud.WBP_PlayerHud_C"))
                (UserInterface|Viewport|AddtoViewport _returnvalue_3 0)
                (Utilities|FlowControl|Delay (Class|WidgetAnimation|GetEndTime (Variables|/Game/Blueprints/Widget/WBP_FadeLevel.WBP_FadeLevel_C|GetFade (Variables|Default|GetWD_Fade))))
                (Widget|RemovefromParent (Variables|Default|GetWD_Fade))))))
        (else
          (Game|LoadStreamLevel(byName) "Area1_livingQuaters" true)
          (bind _returnvalue_4 (SaveGame|CreateSaveGameObject "/Game/Blueprints/BP_SaveGame.BP_SaveGame_C"))
          (Variables|Default|SetSaveGame _returnvalue_4)
          (goto _label))))))

(fn ConstructionScript)