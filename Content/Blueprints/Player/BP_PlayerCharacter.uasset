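; Player character Blueprint handling the pause menu, a debug key that spawns a MadDog AI, radial-damage logging and throw-arc input.
; Q toggles a path-prediction flag while held, and the mouse wheel adjusts the arc.
; Helper functions predict the projectile path from the weapon socket, position an impact marker and build spline meshes along it.
; The EventGraph logic that creates and refreshes this trajectory preview is disconnected, so it never runs.
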(event Game|Damage|EventRadialDamage
  (params (DamageReceived :type Float%20%28single-precision%29) (DamageType :type Damage%20Type%20Object%20Reference) (Origin :type Vector :default "0, 0, 0") (HitInfo :type Hit%20Result%20Structure%20%28by%20ref%29) (InstigatedBy :type Controller%20Object%20Reference) (DamageCauser :type Actor%20Object%20Reference))
  (Development|PrintString (Utilities|GetDisplayName DamageCauser)))

(event Input|ActionEvents|InputActionPauseMenu
  (params (Key :type Key%20Structure :default "None"))
  (bind _returnvalue (Game|GetPlayerController 0))
  (:Pressed
    (bind _returnvalue_2 (UserInterface|CreateWidget "/Game/Blueprints/Widget/WBP_PauseMenu.WBP_PauseMenu_C"))
    (UserInterface|Viewport|AddtoViewport _returnvalue_2 0)
    (Game|SetGamePaused true)
    (Input|SetInputModeUIOnly _returnvalue _returnvalue_2 "DoNotLock")
    (Variables|/Script/Engine.PlayerController|SetbShowMouseCursor _returnvalue true)))

(event Input|MouseEvents|MouseWheelDown
  (params (Key :type Key%20Structure :default "None"))
  (:Pressed
    (Variables|Default|SetArcLength (- (Variables|Default|GetArcLength) 0.01))))

(event Input|KeyboardEvents|K
  (params (Key :type Key%20Structure :default "None")))

(event Input|MouseEvents|MouseWheelUp
  (params (Key :type Key%20Structure :default "None"))
  (:Pressed
    (Variables|Default|SetArcLength (+ (Variables|Default|GetArcLength) 0.01))))

(event Input|KeyboardEvents|Q
  (params (Key :type Key%20Structure :default "None"))
  (:Pressed
    (Variables|Default|SetbPredictPath true))
  (:Released
    (Variables|Default|SetbPredictPath false)))

(event Input|KeyboardEvents|L
  (params (Key :type Key%20Structure :default "None"))
  (:Pressed
    (AI|SpawnAIFromClass "/Game/Blueprints/AI/NPC/MadDog/BP_MadDogNPCAI.BP_MadDogNPCAI_C" "/Game/Blueprints/AI/NPC/MadDog/BT_MadDog.BT_MadDog" "700.000000,400.000000,250.000000" "0, 0, 0" false 0)))

(fn ConstructionScript)