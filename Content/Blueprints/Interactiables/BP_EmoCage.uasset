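; BP_EmoCage is a cage that opens and releases the Emo actors inside it to chase the player.
; BeginPlay waits briefly, then calls the Release event, which plays the OpenCage timeline to rotate StaticMesh1 open.
; When the timeline finishes, every Emo overlapping the Box component is told to ChasePlayer.
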(event Custom|Release
  (bind _newtrack_0 (Timeline|OpenCage Play)
    (:Update
      (Transformation|SetRelativeRotation (Variables|Default|GetStaticMesh1) (Math|Rotator|Lerp(Rotator) "0, 0, 0" "0, 0,-90.000000" _newtrack_0 true) false false))
    (:Finished
      (for _array_element (Collision|GetOverlappingActors (Variables|Default|GetBox) "/Game/Blueprints/AI/NPC/Emo/Emo.Emo_C" :!class /Script/Engine.PrimitiveComponent)
        (bind _asemo (Utilities|Casting|CastToEmo _array_element))
        (Default|ChasePlayer _asemo)))))

(event EventBeginPlay
  (Utilities|FlowControl|Delay 1.0)
  (CallFunction|Release))

(event Collision|EventActorBeginOverlap
  (params (OtherActor :type Actor%20Object%20Reference)))

(event EventTick
  (params (DeltaSeconds :type Float%20%28single-precision%29)))

(fn ConstructionScript)