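; BP_ShieldAmmo is an interactable pickup that restores shield to the player character.
; When its Cube component is overlapped by a PlayerCharacter whose CurrentShield is below a hardcoded 100, it calls HealShield with the AddShield amount and destroys itself.
; Players at or above that threshold leave the pickup in place.
; BeginPlay and the construction script only call their parent implementations.
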(event OnComponentBeginOverlap(Cube)
  (params (OverlappedComponent :type Primitive%20Component%20Object%20Reference) (OtherActor :type Actor%20Object%20Reference) (OtherComp :type Primitive%20Component%20Object%20Reference) (OtherBodyIndex :type Integer) (bFromSweep :type Boolean) (SweepResult :type Hit%20Result%20Structure%20%28by%20ref%29))
  (bind _asplayer_character (Utilities|Casting|CastToPlayerCharacter OtherActor))
  (if (< (Variables|/Script/OnceUponAGamer.PlayerCharacter|GetCurrentShield _asplayer_character) 1e+02)
    (Class|PlayerCharacter|HealShield _asplayer_character (Variables|Default|GetAddShield))
    (Actor|DestroyActor)))

(event EventBeginPlay
  (|CallParentFunction))

(fn ConstructionScript
  (|CallParentFunction))