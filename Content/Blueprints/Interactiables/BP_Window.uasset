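; BP_Window is a window actor with two doors that swing open when its OpenWindow event runs.
; OpenWindow plays the Open timeline, whose track drives SetRotation on both doors toward the same fixed 90-degree relative rotation.
; Each update lerps from the door's current rotation rather than a stored start, so the easing compounds.
; A delayed self-call to OpenWindow is left unconnected, so nothing in this Blueprint triggers the opening.
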(event Custom|OpenWindow
  (bind _newtrack_0 (Timeline|Open Play)
    (:Update
      (CallFunction|SetRotation (Variables|Default|GetWindowDoor1) _newtrack_0)
      (CallFunction|SetRotation (Variables|Default|GetWindowDoor2) _newtrack_0))))

(event EventBeginPlay)

(event Collision|EventActorBeginOverlap
  (params (OtherActor :type Actor%20Object%20Reference)))

(event EventTick
  (params (DeltaSeconds :type Float%20%28single-precision%29)))

(fn ConstructionScript)

(fn SetRotation
  (params (self2 :type Scene%20Component%20Object%20Reference) (Alpha :type Float%20%28single-precision%29))
  (Transformation|SetRelativeRotation self2 (Math|Rotator|Lerp(Rotator) (Variables|/Script/Engine.SceneComponent|GetRelativeRotation self2) "0,90.000000, 0" Alpha) false false))