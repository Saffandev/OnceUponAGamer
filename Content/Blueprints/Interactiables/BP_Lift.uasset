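; Single-trip lift that carries the player from its placed position by the LiftDestination offset.
; Player overlap opens two sliding gates via a timeline, and a panel trigger enables input for the E key.
; Pressing E tints the panel's emissive and reverses the gate timeline, whose Finished event starts the movement timeline.
; On arrival the gates reopen and IsDoorOpen is set, blocking further presses.
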(event OnComponentBeginOverlap(LiftCollision)
  (params (OverlappedComponent :type Primitive%20Component%20Object%20Reference) (OtherActor :type Actor%20Object%20Reference) (OtherComp :type Primitive%20Component%20Object%20Reference) (OtherBodyIndex :type Integer) (bFromSweep :type Boolean) (SweepResult :type Hit%20Result%20Structure%20%28by%20ref%29))
  (if (not (Variables|Default|GetbIsMoving))
    (if (not (Variables|Default|GetbIsDoorOpen))
      (Utilities|Casting|CastToBP_PlayerCharacter OtherActor)
      (CallFunction|OpenLiftDoor))))

(event OnComponentBeginOverlap(NumberPanelCollision)
  (params (OverlappedComponent :type Primitive%20Component%20Object%20Reference) (OtherActor :type Actor%20Object%20Reference) (OtherComp :type Primitive%20Component%20Object%20Reference) (OtherBodyIndex :type Integer) (bFromSweep :type Boolean) (SweepResult :type Hit%20Result%20Structure%20%28by%20ref%29))
  (Utilities|Casting|CastToBP_PlayerCharacter OtherActor)
  (Variables|Default|SetbIsPlayerInsidePanelRadius true)
  (Input|EnableInput (Game|GetPlayerController 0)))

(event OnComponentEndOverlap(NumberPanelCollision)
  (params (OverlappedComponent :type Primitive%20Component%20Object%20Reference) (OtherActor :type Actor%20Object%20Reference) (OtherComp :type Primitive%20Component%20Object%20Reference) (OtherBodyIndex :type Integer))
  (Utilities|Casting|CastToBP_PlayerCharacter OtherActor)
  (Variables|Default|SetbIsPlayerInsidePanelRadius false)
  (Input|DisableInput (Game|GetPlayerController 0)))

(event Custom|OpenLiftDoor
  (bind _toggle_alpha (Timeline|Toggle%20Lift%20Gate Play)
    (:Update
      (Transformation|SetRelativeLocation (Variables|Default|GetSmallliftDoor) (Math|Vector|Lerp(Vector) "204.239059,296.068848,-217.439590" "204.239059,600.741211,-217.439590" _toggle_alpha) false false)
      (Transformation|SetRelativeLocation (Variables|Default|GetSmallliftDoor1) (Math|Vector|Lerp(Vector) "204.238724,-20.060165,-217.439590" "204.238724,-320.840790,-217.439590" _toggle_alpha) false false))
    (:Finished
      (if (Variables|Default|GetbCanInitiateLift)
        (CallFunction|InitiateLift)))))

(event Custom|CloseLiftDoor
  (bind _toggle_alpha (Timeline|Toggle%20Lift%20Gate Reverse)
    (:Update
      (Transformation|SetRelativeLocation (Variables|Default|GetSmallliftDoor) (Math|Vector|Lerp(Vector) "204.239059,296.068848,-217.439590" "204.239059,600.741211,-217.439590" _toggle_alpha) false false)
      (Transformation|SetRelativeLocation (Variables|Default|GetSmallliftDoor1) (Math|Vector|Lerp(Vector) "204.238724,-20.060165,-217.439590" "204.238724,-320.840790,-217.439590" _toggle_alpha) false false))
    (:Finished
      (if (Variables|Default|GetbCanInitiateLift)
        (CallFunction|InitiateLift)))))

(event Custom|InitiateLift
  (bind _newtrack_0 (Timeline|MoveLift Play)
    (:Update
      (Transformation|SetActorLocation (Math|Vector|Lerp(Vector) (Variables|Default|GetLiftSourceLocation) (+ (Variables|Default|GetLiftDestination) (Variables|Default|GetLiftSourceLocation)) _newtrack_0) false false))
    (:Finished
      (CallFunction|OpenLiftDoor)
      (Variables|Default|SetbIsDoorOpen true)
      (Variables|Default|SetbIsMoving false))))

(event EventBeginPlay
  (Variables|Default|SetLiftSourceLocation (Transformation|GetActorLocation))
  (Input|DisableInput (Game|GetPlayerController 0)))

(event Input|KeyboardEvents|E
  (params (Key :type Key%20Structure :default "None"))
  (bind _liftnumberpanel (Variables|Default|GetLiftNumberPanel))
  (:Pressed
    (if (not (Variables|Default|GetbIsDoorOpen))
      (if (Variables|Default|GetbIsPlayerInsidePanelRadius)
        (CallFunction|CloseLiftDoor)
        (Variables|Default|SetbIsMoving true)
        (Variables|Default|SetbCanInitiateLift true)
        (bind _returnvalue (Rendering|Material|CreateDynamicMaterialInstance _liftnumberpanel 2 (Rendering|Material|GetMaterial _liftnumberpanel 2) "None" :!class /Script/Engine.PrimitiveComponent))
        (Rendering|Material|SetVectorParameterValue _returnvalue "Emissive" "(R=10.000000,G=0.416667,B=0.416667,A=1.000000)" :!class /Script/Engine.MaterialInstanceDynamic)))))

(fn ConstructionScript)