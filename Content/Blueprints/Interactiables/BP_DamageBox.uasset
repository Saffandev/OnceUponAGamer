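; BP_DamageBox is an interactable damage volume that repeatedly hurts the player character while it stays inside the box.
; Box overlap by BP_PlayerCharacter applies damage immediately to player 0's character, prints a debug string and starts a looping one-second timer.
; The timer's DamagePlayer event re-enters the same chain, setting the timer again on every tick.
; Ending the overlap clears the stored timer handle to stop the damage.
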(event OnComponentBeginOverlap(Box)
  (params (OverlappedComponent :type Primitive%20Component%20Object%20Reference) (OtherActor :type Actor%20Object%20Reference) (OtherComp :type Primitive%20Component%20Object%20Reference) (OtherBodyIndex :type Integer) (bFromSweep :type Boolean) (SweepResult :type Hit%20Result%20Structure%20%28by%20ref%29))
  (Utilities|Casting|CastToBP_PlayerCharacter OtherActor)
  (Development|PrintString "Damage")
  (Game|Damage|ApplyDamage (Game|GetPlayerCharacter 0) 5.0 0 self)
  (bind _returnvalue (Utilities|Time|SetTimerbyEvent (delegate Custom|DamagePlayer) 1.0 true))
  (Variables|Default|SetdamageHandle _returnvalue))

(event OnComponentEndOverlap(Box)
  (params (OverlappedComponent :type Primitive%20Component%20Object%20Reference) (OtherActor :type Actor%20Object%20Reference) (OtherComp :type Primitive%20Component%20Object%20Reference) (OtherBodyIndex :type Integer))
  (Utilities|Casting|CastToBP_PlayerCharacter OtherActor)
  (Utilities|Time|ClearandInvalidateTimerbyHandle (Variables|Default|GetdamageHandle)))

(event Custom|DamagePlayer
  (Development|PrintString "Damage")
  (Game|Damage|ApplyDamage (Game|GetPlayerCharacter 0) 5.0 0 self)
  (bind _returnvalue (Utilities|Time|SetTimerbyEvent (delegate Custom|DamagePlayer) 1.0 true))
  (Variables|Default|SetdamageHandle _returnvalue))

(event EventBeginPlay)

(event Collision|EventActorBeginOverlap
  (params (OtherActor :type Actor%20Object%20Reference)))

(event EventTick
  (params (DeltaSeconds :type Float%20%28single-precision%29)))

(fn ConstructionScript)