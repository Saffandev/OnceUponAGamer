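; BP_SmallDoor is a small interactable door that builds on a parent door class and shows its lock state.
; On BeginPlay it runs the parent logic, then sets a vertical open location for the door.
; Its ToggleDoor override calls the parent with IsThreat always false, ignoring the input, then swaps the DoorStatus material between locked and unlocked according to LockDoor.
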(event EventBeginPlay
  (|CallParentFunction)
  (Variables|Default|SetOpenDoorLocation "0, 0,150.338821"))

(event Collision|EventActorBeginOverlap
  (params (OtherActor :type Actor%20Object%20Reference))
  (|CallParentFunction OtherActor) ; This node is disabled and will not be called.\nDrag off pins to build functionality.
)

(event EventTick
  (params (DeltaSeconds :type Float%20%28single-precision%29))
  (|CallParentFunction DeltaSeconds) ; This node is disabled and will not be called.\nDrag off pins to build functionality.
)

(fn ConstructionScript
  (|CallParentFunction))

(fn ToggleDoor
  (params (LockDoor :type Boolean) (IsThreat :type Boolean))
  (|CallParentFunction LockDoor false)
  (Rendering|Material|SetMaterial (Variables|Default|GetDoorStatus) 0 (select LockDoor (Variables|Default|GetM_DoorLocked) (Variables|Default|GetM_OpenUnlocked))))