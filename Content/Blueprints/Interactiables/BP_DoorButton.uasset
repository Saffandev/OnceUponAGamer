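; BP_DoorButton is an interactable button that toggles a referenced door and calls Call2ndWave when E is pressed.
; Input starts disabled, turns on when the PlayerCharacter begins overlapping Box, and turns off when it ends overlap with Button rather than Box.
; A press also moves the Button to a fixed pushed-in position and disables input until Box is entered again.
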(event OnComponentBeginOverlap(Box)
  (params (OverlappedComponent :type Primitive%20Component%20Object%20Reference) (OtherActor :type Actor%20Object%20Reference) (OtherComp :type Primitive%20Component%20Object%20Reference) (OtherBodyIndex :type Integer) (bFromSweep :type Boolean) (SweepResult :type Hit%20Result%20Structure%20%28by%20ref%29))
  (Utilities|Casting|CastToPlayerCharacter OtherActor)
  (Input|EnableInput (Game|GetPlayerController 0)))

(event OnComponentEndOverlap(Button)
  (params (OverlappedComponent :type Primitive%20Component%20Object%20Reference) (OtherActor :type Actor%20Object%20Reference) (OtherComp :type Primitive%20Component%20Object%20Reference) (OtherBodyIndex :type Integer))
  (Utilities|Casting|CastToPlayerCharacter OtherActor)
  (Input|DisableInput (Game|GetPlayerController 0)))

(event EventBeginPlay
  (Input|DisableInput (Game|GetPlayerController 0)))

(event Input|KeyboardEvents|E
  (params (Key :type Key%20Structure :default "None"))
  (:Pressed
    (bind _doortointeract (Variables|Default|GetDoorToInteract)
      (:then
        (Default|ToggleDoor _doortointeract false false))
      (:else
        _))
    (Transformation|SetRelativeLocation (Variables|Default|GetButton) "0,2.600000, 0" false false)
    (Input|DisableInput (Game|GetPlayerController 0))
    (Default|Call2ndWave)))

(fn ConstructionScript)