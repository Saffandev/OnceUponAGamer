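; Big interactable door that rises when the player enters its trigger box and acts as a level-streaming gate.
; On overlap, an unlocked door steps through its load and unload level arrays by re-calling LoadUnload, opening once the last load completes.
; The ToggleGate timeline lerps the mesh upward, then reverses when the box's overlap ends or the player is gone shortly after opening.
; ToggleDoor sets the lock state.
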(event OnComponentBeginOverlap(Box)
  (params (OverlappedComponent :type Primitive%20Component%20Object%20Reference) (OtherActor :type Actor%20Object%20Reference) (OtherComp :type Primitive%20Component%20Object%20Reference) (OtherBodyIndex :type Integer) (bFromSweep :type Boolean) (SweepResult :type Hit%20Result%20Structure%20%28by%20ref%29))
  (if (not (Variables|Default|GetbIsLocked))
    (if (not (Variables|Default|GetbIsDoorOpen))
      (Utilities|Casting|CastToPlayerCharacter OtherActor)
      (CallFunction|Load/Unload))))

(event OnComponentEndOverlap(Box)
  (params (OverlappedComponent :type Primitive%20Component%20Object%20Reference) (OtherActor :type Actor%20Object%20Reference) (OtherComp :type Primitive%20Component%20Object%20Reference) (OtherBodyIndex :type Integer))
  (if (Variables|Default|GetbIsDoorOpen)
    (bind (_direction _doortogglealpha) (Timeline|Toggle%20Gate Reverse)
      (:Update
        (Transformation|SetRelativeLocation (Variables|Default|GetDoor) (Math|Vector|Lerp(Vector) (Variables|Default|GetCloseDoorLocation) (Variables|Default|GetOpenDoorLocation) _doortogglealpha) false false))
      (:Finished
        (if (Utilities|Enum|Equal(Enum) _direction "Forward")
          (Variables|Default|SetbIsDoorOpen true)
          (Utilities|FlowControl|Delay 0.5)
          (if (not (Collision|IsOverlappingActor (Variables|Default|GetBox) (Game|GetPlayerCharacter 0) :!class /Script/Engine.PrimitiveComponent))
            (Timeline|Toggle%20Gate Reverse))
          (else
            (Variables|Default|SetbIsDoorOpen false)))))))

(event Custom|Load/Unload
  (Utilities|FlowControl|Sequence
    (:then_0
      (if (== (Utilities|Array|Length (Variables|Default|GetLevelToLoad)) 0)
        (CallFunction|InitDoor)
        (else
          (Class|GameplayStatics|LoadStreamLevelbySoftObjectPtr (Utilities|Array|Get(acopy) (Variables|Default|GetLevelToLoad) (Variables|Default|GetCurrentLevelLoadedNumber)) true false)
          (if (== (Utilities|Array|Length (Variables|Default|GetLevelToLoad)) (+ (Variables|Default|GetCurrentLevelLoadedNumber) 1))
            (Variables|Default|SetCurrentLevelLoadedNumber 0)
            (CallFunction|InitDoor)
            (else
              (Math|Integer|IncrementInt (Variables|Default|GetCurrentLevelLoadedNumber)
                (:%20%20
                  (CallFunction|Load/Unload))))))))
    (:then_1
      (if (not (== (Utilities|Array|Length (Variables|Default|GetLevelToUnload)) 0))
        (Class|GameplayStatics|UnloadStreamLevelbySoftObjectPtr (Utilities|Array|Get(acopy) (Variables|Default|GetLevelToUnload) (Variables|Default|GetCurrentLevelUnloadedNumber)) false)
        (if (== (Utilities|Array|Length (Variables|Default|GetLevelToUnload)) (+ (Variables|Default|GetCurrentLevelUnloadedNumber) 1))
          (Variables|Default|SetCurrentLevelUnloadedNumber 0)
          (else
            (Math|Integer|IncrementInt (Variables|Default|GetCurrentLevelUnloadedNumber)
              (:%20%20
                (CallFunction|Load/Unload)))))))))

(event Custom|InitDoor
  (bind (_direction _doortogglealpha) (Timeline|Toggle%20Gate Play)
    (:Update
      (Transformation|SetRelativeLocation (Variables|Default|GetDoor) (Math|Vector|Lerp(Vector) (Variables|Default|GetCloseDoorLocation) (Variables|Default|GetOpenDoorLocation) _doortogglealpha) false false))
    (:Finished
      (if (Utilities|Enum|Equal(Enum) _direction "Forward")
        (Variables|Default|SetbIsDoorOpen true)
        (Utilities|FlowControl|Delay 0.5)
        (if (not (Collision|IsOverlappingActor (Variables|Default|GetBox) (Game|GetPlayerCharacter 0) :!class /Script/Engine.PrimitiveComponent))
          (Timeline|Toggle%20Gate Reverse))
        (else
          (Variables|Default|SetbIsDoorOpen false))))))

(event EventBeginPlay
  (Variables|Default|SetCloseDoorLocation (Variables|/Script/Engine.SceneComponent|GetRelativeLocation (Variables|Default|GetDoor)))
  (Variables|Default|SetOpenDoorLocation "0, 0,920.541870"))

(event Collision|EventActorBeginOverlap
  (params (OtherActor :type Actor%20Object%20Reference)))

(event EventTick
  (params (DeltaSeconds :type Float%20%28single-precision%29)))

(fn ConstructionScript)

(fn ToggleDoor
  (params (LockDoor :type Boolean))
  (Variables|Default|SetbIsLocked LockDoor))