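; A one-shot interactable box that releases a health pickup and a shield pickup when it takes point damage.
; The first hit disables further damage and spawns BP_HealthAmmo at the Arrow, then BP_ShieldAmmo after a short delay.
; A shared Spawn event launches the current pickup along the arrow's forward vector while a timeline scales it up from zero.
; A second timeline then drives the spotlight's intensity as a fade-out.
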(event Custom|Spawn
  (bind _health (Variables|Default|GetHealth))
  (Variables|/Game/Blueprints/Interactiables/BP_HealthAmmo.BP_HealthAmmo_C|SetbIsSpawned _health false)
  (Physics|AddImpulse (Variables|/Game/Blueprints/Interactiables/BP_HealthAmmo.BP_HealthAmmo_C|GetCube _health) (* (Math|Rotator|GetRotationXVector (Transformation|GetWorldRotation (Variables|Default|GetArrow))) 2e+02) "None" true)
  (bind _newtrack_0 (Timeline|Timeline_0 Play)
    (:Update
      (Transformation|SetActorScale3D (Variables|Default|GetHealth) (Math|Vector|Lerp(Vector) "0, 0, 0" "0.040000,0.040000,0.040000" _newtrack_0)))))

(event EventBeginPlay)

(event Collision|EventActorBeginOverlap
  (params (OtherActor :type Actor%20Object%20Reference)))

(event EventTick
  (params (DeltaSeconds :type Float%20%28single-precision%29)))

(event Game|Damage|EventPointDamage
  (params (Damage :type Float%20%28single-precision%29) (DamageType :type Damage%20Type%20Object%20Reference) (HitLocation :type Vector :default "0, 0, 0") (HitNormal :type Vector :default "0, 0, 0") (HitComponent :type Primitive%20Component%20Object%20Reference) (BoneName :type Name :default "None") (ShotFromDirection :type Vector :default "0, 0, 0") (InstigatedBy :type Controller%20Object%20Reference) (DamageCauser :type Actor%20Object%20Reference) (HitInfo :type Hit%20Result%20Structure%20%28by%20ref%29))
  (bind _arrow (Variables|Default|GetArrow))
  (bind _arrow_2 (Variables|Default|GetArrow))
  (bind _returnvalue (Transformation|GetWorldLocation _arrow_2))
  (bind _returnvalue_2 (Transformation|GetWorldRotation _arrow))
  (Variables|Actor|SetbCanBeDamaged false)
  (bind _returnvalue_3 (Game|SpawnActorfromClass "/Game/Blueprints/Interactiables/BP_HealthAmmo.BP_HealthAmmo_C" (Math|Transform|MakeTransform _returnvalue _returnvalue_2 "0.000000,0.000000,0.000000") "Undefined" 0 false 0))
  (bind _output_get (Variables|Default|SetHealth _returnvalue_3))
  (Variables|/Game/Blueprints/Interactiables/BP_HealthAmmo.BP_HealthAmmo_C|SetAddHealth _output_get 1e+02)
  (CallFunction|Spawn)
  (Utilities|FlowControl|Delay 0.4)
  (bind _returnvalue_4 (Game|SpawnActorfromClass "/Game/Blueprints/Interactiables/BP_ShieldAmmo.BP_ShieldAmmo_C" (Math|Transform|MakeTransform _returnvalue _returnvalue_2 "0.000000,0.000000,0.000000") "Undefined" 0 false 0))
  (bind _output_get_2 (Variables|Default|SetHealth _returnvalue_4))
  (Variables|/Game/Blueprints/Interactiables/BP_HealthAmmo.BP_HealthAmmo_C|SetAddShield _output_get_2 1e+02)
  (CallFunction|Spawn)
  (bind _newtrack_0 (Timeline|FadeOut Play)
    (:Update
      (Rendering|Components|Light|SetIntensity (Variables|Default|GetSpotLight) _newtrack_0))))

(fn ConstructionScript)