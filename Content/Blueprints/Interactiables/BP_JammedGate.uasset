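; A jammed double gate that the player forces open by repeatedly pressing E while standing in its trigger box.
; Box overlaps toggle player input on the gate, and each press nudges the two doors apart along X.
; Tick eases both doors back toward their starting positions until either nears its final location.
; That marks the gate opened, stopping the pull-back and quickly interpolating both doors to their open positions.
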(event OnComponentBeginOverlap(Box)
  (params (OverlappedComponent :type Primitive%20Component%20Object%20Reference) (OtherActor :type Actor%20Object%20Reference) (OtherComp :type Primitive%20Component%20Object%20Reference) (OtherBodyIndex :type Integer) (bFromSweep :type Boolean) (SweepResult :type Hit%20Result%20Structure%20%28by%20ref%29))
  (Utilities|Casting|CastToPlayerCharacter OtherActor)
  (Variables|Default|SetbIsPlayerInBox true)
  (Input|EnableInput (Game|GetPlayerController 0)))

(event OnComponentEndOverlap(Box)
  (params (OverlappedComponent :type Primitive%20Component%20Object%20Reference) (OtherActor :type Actor%20Object%20Reference) (OtherComp :type Primitive%20Component%20Object%20Reference) (OtherBodyIndex :type Integer))
  (Utilities|Casting|CastToPlayerCharacter OtherActor)
  (Variables|Default|SetbIsPlayerInBox false)
  (Input|DisableInput (Game|GetPlayerController 0)))

(event EventBeginPlay
  (Variables|Default|SetDoor1InitialLoc (Variables|/Script/Engine.SceneComponent|GetRelativeLocation (Variables|Default|GetDoor1)))
  (Variables|Default|SetDoor2InitialLoc (Variables|/Script/Engine.SceneComponent|GetRelativeLocation (Variables|Default|GetDoor2)))
  (Input|DisableInput (Game|GetPlayerController 0)))

(event EventTick
  (params (DeltaSeconds :type Float%20%28single-precision%29))
  (bind _door2initialloc (Variables|Default|GetDoor2InitialLoc))
  (bind _door1 (Variables|Default|GetDoor1))
  (bind _door2 (Variables|Default|GetDoor2))
  (bind _door1initialloc (Variables|Default|GetDoor1InitialLoc))
  (bind _relativelocation (Variables|/Script/Engine.SceneComponent|GetRelativeLocation _door2))
  (bind _relativelocation_2 (Variables|/Script/Engine.SceneComponent|GetRelativeLocation _door1))
  (Utilities|FlowControl|Sequence
    (:then_0
      (if (not (Variables|Default|GetbIsdoorOpened))
        (if (not (Math|Vector|Equal(Vector) _relativelocation_2 _door1initialloc 0.0001))
          (Transformation|SetRelativeLocation (Variables|Default|GetDoor1) (Math|Interpolation|VInterpTo _relativelocation_2 _door1initialloc (Utilities|Time|GetWorldDeltaSeconds) 2.0) false false))))
    (:then_1
      (if (not (Variables|Default|GetbIsdoorOpened))
        (if (not (Math|Vector|Equal(Vector) _relativelocation _door2initialloc 0.0001))
          (Transformation|SetRelativeLocation (Variables|Default|GetDoor2) (Math|Interpolation|VInterpTo _relativelocation _door2initialloc (Utilities|Time|GetWorldDeltaSeconds) 2.0) false false))))
    (:then_2
      (if (Math|Vector|Equal(Vector) (Variables|/Script/Engine.SceneComponent|GetRelativeLocation (Variables|Default|GetDoor1)) (Variables|Default|GetDoor1FinalLoc) 4e+01)
        (Variables|Default|SetbIsdoorOpened true :!label _label)
        (Transformation|SetRelativeLocation (Variables|Default|GetDoor1) (Math|Interpolation|VInterpTo (Variables|/Script/Engine.SceneComponent|GetRelativeLocation (Variables|Default|GetDoor1)) (Variables|Default|GetDoor1FinalLoc) (Utilities|Time|GetWorldDeltaSeconds) 2e+01) false false)
        (Transformation|SetRelativeLocation (Variables|Default|GetDoor2) (Math|Interpolation|VInterpTo (Variables|/Script/Engine.SceneComponent|GetRelativeLocation (Variables|Default|GetDoor2)) (Variables|Default|GetDoor2FinalLoc) (Utilities|Time|GetWorldDeltaSeconds) 2e+01) false false)))
    (:then_3
      (if (Math|Vector|Equal(Vector) (Variables|/Script/Engine.SceneComponent|GetRelativeLocation (Variables|Default|GetDoor2)) (Variables|Default|GetDoor2FinalLoc) 5e+01)
        (goto _label)))))

(event Input|KeyboardEvents|E
  (params (Key :type Key%20Structure :default "None"))
  (bind _door1 (Variables|Default|GetDoor1))
  (bind _door2 (Variables|Default|GetDoor2))
  (bind _relativelocation (Variables|/Script/Engine.SceneComponent|GetRelativeLocation _door2))
  (bind _relativelocation_2 (Variables|/Script/Engine.SceneComponent|GetRelativeLocation _door1))
  (:Pressed
    (if (not (Variables|Default|GetbIsdoorOpened))
      (if (Variables|Default|GetbIsPlayerInBox)
        (Transformation|SetRelativeLocation (Variables|Default|GetDoor1) (Math|Vector|MakeVector (- (.x _relativelocation_2) 2e+01) (.y _relativelocation_2) (.z _relativelocation_2)) false false)
        (Transformation|SetRelativeLocation (Variables|Default|GetDoor2) (Math|Vector|MakeVector (+ (.x _relativelocation) 2e+01) (.y _relativelocation) (.z _relativelocation)) false false)))))

(fn ConstructionScript)