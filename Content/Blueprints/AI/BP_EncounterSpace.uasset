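; BP_EncounterSpace is an AI encounter area that locks its gates around the player during a threat and reopens them when cleared.
; The player overlapping ThreatDetector fires Threat once, locking every gate and, in boss rooms, calling the Mad Dog doors.
; TheratCleared unlocks the gates when no further wave is flagged or the current wave equals the total.
; In multi-wave boss rooms, it also triggers boss initialization once.
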(event OnComponentBeginOverlap(ThreatDetector)
  (params (OverlappedComponent :type Primitive%20Component%20Object%20Reference) (OtherActor :type Actor%20Object%20Reference) (OtherComp :type Primitive%20Component%20Object%20Reference) (OtherBodyIndex :type Integer) (bFromSweep :type Boolean) (SweepResult :type Hit%20Result%20Structure%20%28by%20ref%29))
  (if (== OtherActor (Game|GetPlayerCharacter 0))
    (CallFunction|Threat)))

(event Custom|Threat
  (Utilities|FlowControl|DoOnce false
    (:Completed
      (Utilities|FlowControl|Sequence
        (:then_0
          (for _array_element (Variables|Default|GetGates)
            (Default|ToggleDoor _array_element true true)))
        (:then_1
          (if (Variables|Default|GetbIsBossRoom)
            (Default|CallMadDogDoors)))))))

(event EventTheratCleared
  (if (Variables|Default|GetbIsAnotherWave)
    (if (Variables|Default|GetbIsBossRoom)
      (Utilities|FlowControl|Sequence
        (:then_0
          (Utilities|FlowControl|DoOnce false
            (:Completed
              (Default|CallInitBossTrigger))))
        (:then_1
          (if (== (Variables|Default|GetCurrentWave) (Variables|Default|GetTotalWaves)) :!label _label
            (for _array_element (Variables|Default|GetGates) :!label _label_2
              (Utilities|IsValid _array_element
                (:Is%20Valid
                  (Default|ToggleDoor _array_element false false)))))))
      (else
        (goto _label)))
    (else
      (goto _label_2))))

(event EventThreatDetected)

(event EventSomeoneIsDead)

(fn ConstructionScript)