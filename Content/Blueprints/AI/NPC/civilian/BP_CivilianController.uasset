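; AI controller for civilian NPCs that wander at random and flee from perceived stimuli.
; A looping timer moves the pawn to random nearby navmesh points.
; A perception update, throttled by a DoOnce, stops roaming, raises walk speed and runs toward a navmesh point away from the stimulus, resuming roaming after a retriggerable delay.
; SafetyLocation picks that point with debug spheres; its rotating retry search is disconnected.
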(event OnTargetPerceptionUpdated(AIPerception)
  (params (Actor :type Actor%20Object%20Reference) (Stimulus :type AI%20Stimulus%20Structure))
  (Utilities|FlowControl|Sequence
    (:then_0
      (Utilities|FlowControl|DoOnce false :!label _label
        (:Completed
          (Variables|Default|SetStimulus Stimulus)
          (Utilities|Time|ClearandInvalidateTimerbyHandle (Variables|Default|GetMoveTimer))
          (Variables|/Script/Engine.CharacterMovementComponent|SetMaxWalkSpeed (Variables|/Script/Engine.Character|GetCharacterMovement (.AsCharacter (Utilities|Casting|CastToCharacter (Pawn|GetControlledPawn)))) 5e+02)
          (bind (_returnvalue _returnvalue2) (|SafetyLocation)
            (:exec
              (if _returnvalue2
                (AI|Navigation|SimpleMovetoLocation self _returnvalue)
                (Utilities|FlowControl|RetriggerableDelay 8.0)
                (Variables|/Script/Engine.CharacterMovementComponent|SetMaxWalkSpeed (Variables|/Script/Engine.Character|GetCharacterMovement (Variables|Default|GetAs%20BP%20Civilian)) 1.8e+02)
                (CallFunction|Roaming)
                (CallFunction|RoamingTimer)))))))
    (:then_1
      (Utilities|FlowControl|Delay 1.0)
      (goto _label Reset))))

(event Custom|Roaming
  (AI|Navigation|MovetoLocation (.RandomLocation (Class|NavigationSystemV1|GetRandomPointinNavigableRadius (Transformation|GetActorLocation (Pawn|GetControlledPawn)) 1e+03 0 0)) -1.0 true true false true 0))

(event Custom|RoamingTimer
  (bind _returnvalue (Utilities|Time|SetTimerbyFunctionName 0 "Roaming" 3.0 true))
  (Variables|Default|SetMoveTimer _returnvalue))

(event EventBeginPlay
  (CallFunction|Roaming)
  (CallFunction|RoamingTimer)
  (bind _asbp_civilian (Utilities|Casting|CastToBP_Civilian (Pawn|GetControlledPawn)))
  (Variables|Default|SetAs%20BP%20Civilian _asbp_civilian))

(fn ConstructionScript)

(fn OwnerDied)