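; BP_Civilian is a civilian NPC that takes damage, dies into a ragdoll and reports violence.
; On AnyDamage it registers a hit at the damage causer's location, then subtracts from Health.
; At zero Health it stops moving, detaches its controller, simulates physics on the mesh and disables capsule collision.
; It also registers a CivilianKilled event at its own location, attributed to the instigator.
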(event Game|Damage|EventAnyDamage
  (params (Damage :type Float%20%28single-precision%29) (DamageType :type Damage%20Type%20Object%20Reference) (InstigatedBy :type Controller%20Object%20Reference) (DamageCauser :type Actor%20Object%20Reference))
  (Utilities|IsValid DamageCauser
    (:Is%20Valid
      (Class|ViolenceRegistration|RegisterViolence self (Transformation|GetActorLocation DamageCauser) InstigatedBy "EVT_HittedSomethingDamaging"))
    (:Is%20Not%20Valid
      _))
  (bind _output_get (Variables|Default|SetHealth (- (Variables|Default|GetHealth) Damage)))
  (if (<= _output_get 0.0)
    (Variables|Actor|SetbCanBeDamaged false)
    (Components|Movement|StopMovementImmediately (Variables|Character|GetCharacterMovement))
    (Class|Pawn|DetachfromControllerPendingDestroy)
    (Physics|SetSimulatePhysics (Variables|Character|GetMesh) true)
    (Class|ViolenceRegistration|RegisterViolence self (Transformation|GetActorLocation) InstigatedBy "EVT_CivilianKilled")
    (Collision|SetCollisionEnabled (Variables|Collision|GetCapsuleComponent) "NoCollision")))

(fn ConstructionScript)