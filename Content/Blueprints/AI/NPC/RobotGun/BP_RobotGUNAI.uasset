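; Robot gun NPC AI that roams and shoots at the player.
; Every five seconds an EQS query supplies move locations; separate random picks drive movement, debug print and sphere.
; A fast looping Fire timer checks line of sight, sets IsShooting, line traces and applies small point damage on player hits.
; The fire montage and the muzzle spread math in Start & End Point are unconnected.
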(event Custom|Fire
  (bind (_returnvalue _returnvalue2) (|Start&EndPoint))
  (bind _output_get (Variables|Default|SetbCanFocus (Controller|LineOfSightTo (Pawn|GetController) (Game|Player|GetPlayerPawn 0) "0, 0, 0" false)))
  (if _output_get
    (Variables|Default|SetbIsShooting true)
    (bind (_outhit _returnvalue_2) (Collision|LineTraceByChannel _returnvalue _returnvalue2 "TraceTypeQuery1" false (Utilities|Array|MakeArray self) "None"))
    (if _returnvalue_2
      (|Damage _outhit))
    (else
      (Variables|Default|SetbIsShooting false))))

(event Custom|MoveTimer
  (bind _returnvalue (AI|EQS|RunEQSQuery "/Game/Blueprints/AI/NPC/RobotGun/EQS_RobotGunMovement.EQS_RobotGunMovement" self "RandomBest5Pct"))
  (EventDispatchers|BindEventtoOnQueryFinishedEvent _returnvalue (delegate Custom|CustomEvent_0)))

(event Custom|CustomEvent_0
  (params (QueryInstance :type Env%20Query%20Instance%20Blueprint%20Wrapper%20Object%20Reference) (QueryStatus :type EEnvQueryStatus%20Enum :default "Processing"))
  (bind _resultlocations (AI|EQS|GetQueryResultsasLocations QueryInstance))
  (AI|Navigation|SimpleMovetoLocation (Pawn|GetController) (Utilities|Array|Get(acopy) _resultlocations (Math|Random|RandomIntegerinRange 0 (- (Utilities|Array|Length _resultlocations) 1))))
  (Development|PrintString (Utilities|String|ToString(Vector) (Utilities|Array|Get(acopy) _resultlocations (Math|Random|RandomIntegerinRange 0 (- (Utilities|Array|Length _resultlocations) 1)))))
  (Rendering|Debug|DrawDebugSphere (Utilities|Array|Get(acopy) _resultlocations (Math|Random|RandomIntegerinRange 0 (- (Utilities|Array|Length _resultlocations) 1))) 1e+02 12 "(R=1.000000,G=0.021217,B=0.000000,A=1.000000)" 5.0))

(event EventBeginPlay
  (Utilities|Time|SetTimerbyEvent (delegate Custom|MoveTimer) 5.0 true)
  (Utilities|Time|SetTimerbyFunctionName 0 "Fire" 0.1 true))

(fn ConstructionScript)