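; Wall turret enemy that deploys from behind sliding doors when the player first enters its trigger box, supporting ground or inverted mounting.
; Timelines open the doors and extend the base, then Tick traces to the player, updates a laser beam and aims base and gun.
; Randomized timers toggle bursts of hitscan point damage.
; Lost health scales smoke and spark particles; death stops ticking, spawns effects and tilts the gun limp.
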(event OnComponentBeginOverlap(TriggerBox)
  (params (OverlappedComponent :type Primitive%20Component%20Object%20Reference) (OtherActor :type Actor%20Object%20Reference) (OtherComp :type Primitive%20Component%20Object%20Reference) (OtherBodyIndex :type Integer) (bFromSweep :type Boolean) (SweepResult :type Hit%20Result%20Structure%20%28by%20ref%29))
  (Utilities|Casting|CastToPlayerCharacter OtherActor)
  (Utilities|FlowControl|DoOnce false
    (:Completed
      (CallFunction|InitiateDoor))))

(event Custom|Initiate_Door
  (bind _torrentd1 (Variables|Default|GetTorrentD1))
  (bind _torrentd2 (Variables|Default|GetTorrentD2))
  (bind _relativelocation (Variables|/Script/Engine.SceneComponent|GetRelativeLocation _torrentd2))
  (bind _relativelocation_2 (Variables|/Script/Engine.SceneComponent|GetRelativeLocation _torrentd1))
  (bind (_x _y _z) (Math|Vector|BreakVector _relativelocation_2))
  (bind (_x_2 _y_2 _z_2) (Math|Vector|BreakVector _relativelocation))
  (bind _window (Variables|Default|GetWindow)
    (:then
      (Default|OpenWindow _window)
      (bind _newtrack_0 (Timeline|Initiatedoor PlayFromStart)
        (:Update
          (Transformation|SetRelativeLocation (Variables|Default|GetTorrentD1) (Math|Vector|Lerp(Vector) _relativelocation_2 (Math|Vector|MakeVector 84.0 _y _z) _newtrack_0) false false)
          (Transformation|SetRelativeLocation (Variables|Default|GetTorrentD2) (Math|Vector|Lerp(Vector) _relativelocation (Math|Vector|MakeVector -84.0 _y_2 _z_2) _newtrack_0) false false))
        (:Finished
          (Audio|PlaySoundatLocation "/Game/Sounds/WallTurrentDOwn_Cue.WallTurrentDOwn_Cue" (Transformation|GetActorLocation) "0, 0, 0" 1.0 1.0 0.0 0 0 0)
          (bind _newtrack_0_2 (Timeline|InitiateTurrent PlayFromStart)
            (:Update
              (Transformation|SetRelativeLocation (Variables|Default|GetBase) (Math|Vector|Lerp(Vector) (Variables|/Script/Engine.SceneComponent|GetRelativeLocation (Variables|Default|GetBase)) "0, 0,140.000000" _newtrack_0_2) false false))
            (:Finished
              (Variables|Default|SetbCanTarget true)
              (bind _smoke (Variables|Default|GetSmoke)
                (:then
                  (Effects|Components|ParticleSystem|SetFloatParameter _smoke "SpawnRate" 0.0))
                (:else
                  _))
              (bind _sparkp (Variables|Default|GetSparkP)
                (:then
                  (Effects|Components|ParticleSystem|SetFloatParameter _sparkp "SpawnRateParticle" 0.0)
                  (Effects|Components|ParticleSystem|SetFloatParameter _sparkp "SpawnRateSpark" 0.0))
                (:else
                  _))
              (bind _returnvalue (Effects|SpawnEmitterAttached "/Game/Particles/P_Laser.P_Laser" (Variables|Default|GetArrow) "None"))
              (Variables|Default|SetLaser _returnvalue))))))
    (:else
      (Timeline|Initiatedoor PlayFromStart))))

(event Custom|DeathRituals
  (bind _deathspark (Variables|Default|GetDeathSpark))
  (bind _returnvalue (Transformation|GetWorldLocation _deathspark))
  (Variables|Actor|SetbCanBeDamaged false)
  (Effects|SpawnEmitteratLocation "/Game/Particles/P_Spark.P_Spark" _returnvalue)
  (bind _returnvalue_2 (Effects|SpawnEmitteratLocation "/Game/StarterContent/Particles/P_Smoke.P_Smoke" _returnvalue))
  (Effects|Components|ParticleSystem|SetFloatParameter _returnvalue_2 "SpawnRate" 6.0)
  (Effects|SpawnEmitteratLocation "/Game/StarterContent/Particles/P_Sparks.P_Sparks" _returnvalue)
  (Audio|PlaySoundatLocation "/Game/Sounds/ShotCircut_Cue.ShotCircut_Cue" (Transformation|GetActorLocation) "0, 0, 0" 1.0 1.0 0.0 0 0 0)
  (bind _laser (Variables|Default|GetLaser)
    (:then
      (Components|DestroyComponent _laser)
      (bind _newtrack_0 (Timeline|DeadGun PlayFromStart)
        (:Update
          (Transformation|SetRelativeRotation (Variables|Default|GetGun) (Math|Rotator|MakeRotator (Math|Float|Lerp (.roll (Variables|/Script/Engine.SceneComponent|GetRelativeRotation (Variables|Default|GetGun))) (select (Variables|Default|GetbIsOnGround) 2e+01 -85.0) _newtrack_0) 0.0 0.0) false false))))
    (:else)))

(event Custom|start%20fire
  ;[1 1 1] Start Shooting
  (if (Variables|Default|GetbCanShoot)
    (|Damage)))

(event Custom|StopFiring
  ;[1 1 1] Stop Shooting
  (Utilities|FlowControl|FlipFlop
    (:A
      (Variables|Default|SetbCanShoot false))
    (:B
      (Variables|Default|SetbCanShoot true))))

(event EventBeginPlay)

(event Collision|EventActorBeginOverlap
  (params (OtherActor :type Actor%20Object%20Reference)))

(event EventTick
  (params (DeltaSeconds :type Float%20%28single-precision%29))
  (bind _arrow (Variables|Default|GetArrow))
  (bind _returnvalue (Transformation|GetWorldLocation _arrow))
  (if (Variables|Default|GetbCanTarget)
    (bind _outhit (Collision|LineTraceByChannel _returnvalue (Transformation|GetActorLocation (Game|GetPlayerCharacter 0)) "TraceTypeQuery1" false (Utilities|Array|MakeArray self) "None"))
    (bind _laser (Variables|Default|GetLaser)
      (:then
        (Class|ParticleSystemComponent|SetBeamSourcePoint _laser 0 _returnvalue)
        (Class|ParticleSystemComponent|SetBeamTargetPoint _laser 0 (.ImpactPoint (Collision|BreakHitResult _outhit))))
      (:else
        _))
    (if (== (.HitActor (Collision|BreakHitResult _outhit)) (Game|GetPlayerCharacter 0))
      (|TurrentRotation)
      ;[1 1 1] Start Shooting
      (if (Utilities|Time|IsTimerActivebyHandle (Variables|Default|GetFireTimer))
        _
        (else
          (bind _returnvalue_2 (Utilities|Time|SetTimerbyEvent (delegate Custom|start%20fire) (Math|Random|RandomFloatinRange 0.08 0.1)))
          (Variables|Default|SetFireTimer _returnvalue_2)))
      ;[1 1 1] Stop Shooting
      (if (not (Utilities|Time|IsTimerActivebyHandle (Variables|Default|GetStopFireTimer)))
        (bind _returnvalue_3 (Utilities|Time|SetTimerbyEvent (delegate Custom|StopFiring) (select (Variables|Default|GetbCanShoot) (Math|Random|RandomFloatinRange 1.7 2.0) (Math|Random|RandomFloatinRange 0.8 1.0))))
        (Variables|Default|SetStopFireTimer _returnvalue_3)))))

(event Game|Damage|EventAnyDamage
  (params (Damage :type Float%20%28single-precision%29) (DamageType :type Damage%20Type%20Object%20Reference) (InstigatedBy :type Controller%20Object%20Reference) (DamageCauser :type Actor%20Object%20Reference))
  (bind _sparkp (Variables|Default|GetSparkP))
  (if (Variables|Default|GetbIsAlive)
    (Utilities|FlowControl|Sequence
      (:then_0
        (Variables|Default|SetHealth (- (Variables|Default|GetHealth) Damage)))
      (:then_1
        (bind _newvalue (CallFunction|ParticlePercentage 6.0))
        (Effects|Components|ParticleSystem|SetFloatParameter (Variables|Default|GetSmoke) "SpawnRate" _newvalue) ; 6
        (bind _newvalue_2 (CallFunction|ParticlePercentage 12.0))
        (Effects|Components|ParticleSystem|SetFloatParameter _sparkp "SpawnRateSpark" _newvalue_2) ; 12
        (bind _newvalue_3 (CallFunction|ParticlePercentage 2e+02))
        (Effects|Components|ParticleSystem|SetFloatParameter _sparkp "SpawnRateParticle" _newvalue_3) ; 100
      )
      (:then_2
        (if (<= (Variables|Default|GetHealth) 0.0)
          (Variables|Default|SetbIsAlive false)
          (Actor|Tick|SetActorTickEnabled false)
          (CallFunction|DeathRituals))))))

(fn ConstructionScript
  (Transformation|SetRelativeLocation (Variables|Default|GetTriggerBox) (Variables|Default|GetBoxLoc) false false))

(fn ParticlePercentage
  (params (ParticleMaxRange :type Float%20%28single-precision%29))
  (bind _output_get (Variables|Default|SetHealthPercentLeft (* (/ (- 1e+02 (Variables|Default|GetHealth)) 1e+02) 1e+02)))
  (return (/ (* _output_get ParticleMaxRange) 1e+02)))

(fn IsDead
  (return (not (Variables|Default|GetbIsAlive))))