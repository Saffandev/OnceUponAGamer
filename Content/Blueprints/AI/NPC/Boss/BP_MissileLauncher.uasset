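; Boss missile launcher actor that fires repeating bursts of three homing missiles from its own transform, with fire sound and muzzle flash.
; StartSpawnTimer runs a looping timer into SpawnMissile, which counts shots, then clears the timer and schedules StartSpawnTimer again after a pause.
; Nothing in this graph starts the cycle, as BeginPlay and Tick are empty and the delayed start and player-facing rotation nodes are disconnected.
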(event Custom|SpawnMissile
  (bind _returnvalue (Transformation|GetActorLocation))
  (if (< (Variables|Default|GetSpawnCount) 3)
    (Math|Integer|IncrementInt (Variables|Default|GetSpawnCount)
      (:%20%20
        (Game|SpawnActorfromClass "/Game/Blueprints/Guns/BP_HomingMissile.BP_HomingMissile_C" (Transformation|GetActorTransform) "Undefined" self 0)
        (Audio|PlaySoundatLocation "/Game/MilitaryWeapDark/Sound/RocketLauncher/RocketLauncherB_Fire_Cue.RocketLauncherB_Fire_Cue" _returnvalue "0, 0, 0" 1.0 1.0 0.0 0 0 0)
        (Effects|SpawnEmitteratLocation "/Game/SciFiWeapLight/FX/Particles/P_RocketLauncher_MuzzleFlash_Front_Dark.P_RocketLauncher_MuzzleFlash_Front_Dark" _returnvalue (Transformation|GetActorRotation))))
    (else
      (Utilities|Time|ClearandInvalidateTimerbyHandle (Variables|Default|GetSpawnTimer))
      (Utilities|Time|SetTimerbyFunctionName 0 "StartSpawnTimer" 3.0)
      (Variables|Default|SetSpawnCount 0))))

(event Custom|StartSpawnTimer
  (bind _returnvalue (Utilities|Time|SetTimerbyEvent (delegate Custom|SpawnMissile) 1.0 true))
  (Variables|Default|SetSpawnTimer _returnvalue))

(event EventBeginPlay)

(event EventTick
  (params (DeltaSeconds :type Float%20%28single-precision%29)))

(fn ConstructionScript)