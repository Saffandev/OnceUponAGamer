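; Boss turret actor that tracks the player when targeting is enabled, yawing its body and rolling its gun at rates that depend on angular error.
; Once fire is initiated, a looping timer runs line-trace shots with point damage and muzzle flash in repeating bursts separated by pauses.
; Lost health scales smoke and sparks; death stops tick, spawns effects and tilts the gun according to ground mounting.
; The startup chain enabling targeting and fire is disconnected.
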(event Custom|DeathRituals
  (bind _deathspark (Variables|Default|GetDeathSpark))
  (bind _returnvalue (Transformation|GetWorldLocation _deathspark))
  (Variables|Actor|SetbCanBeDamaged false)
  (Effects|SpawnEmitteratLocation "/Game/Particles/P_Spark.P_Spark" _returnvalue)
  (bind _returnvalue_2 (Effects|SpawnEmitteratLocation "/Game/StarterContent/Particles/P_Smoke.P_Smoke" _returnvalue))
  (Effects|Components|ParticleSystem|SetFloatParameter _returnvalue_2 "SpawnRate" 6.0)
  (Effects|SpawnEmitteratLocation "/Game/StarterContent/Particles/P_Sparks.P_Sparks" _returnvalue)
  (Audio|PlaySoundatLocation "/Game/Sounds/ShotCircut_Cue.ShotCircut_Cue" (Transformation|GetActorLocation) "0, 0, 0" 1.0 1.0 0.0 0 0 0)
  (bind _laser (Variables|Default|GetLaser)
    (:then
      (Components|DestroyComponent _laser)
      (bind _newtrack_0 (Timeline|DeadGun PlayFromStart)
        (:Update
          (Transformation|SetRelativeRotation (Variables|Default|GetGun) (Math|Rotator|MakeRotator (Math|Float|Lerp (.roll (Variables|/Script/Engine.SceneComponent|GetRelativeRotation (Variables|Default|GetGun))) (select (Variables|Default|GetbIsOnGround) 2e+01 -85.0) _newtrack_0) 0.0 0.0) false false))))
    (:else)))

(event Custom|InitiateFire
  ;[1 1 1] Start Shooting
  (Audio|Components|Audio|Play (Variables|Default|GetInitFire) 0.0)
  (bind _returnvalue (Utilities|Time|SetTimerbyEvent (delegate Custom|start%20fire) 0.06 true 0.7))
  (Variables|Default|SetFireTimer _returnvalue)
  (Utilities|Time|SetTimerbyFunctionName 0 "StopFiring" 4.0))

(event Custom|start%20fire
  ;[1 1 1] Start Shooting
  (|Damage))

(event Custom|StopFiring
  ;[1 1 1] Stop Shooting
  (Audio|Components|Audio|Stop (Variables|Default|GetInitFire))
  (Audio|Components|Audio|Play (Variables|Default|GetStopFire) 0.0)
  (Utilities|Time|ClearandInvalidateTimerbyHandle (Variables|Default|GetFireTimer))
  (Utilities|FlowControl|Delay 2.0)
  (CallFunction|InitiateFire))

(event EventTick
  (params (DeltaSeconds :type Float%20%28single-precision%29))
  (if (Variables|Default|GetbCanTarget)
    (|TurrentRotation DeltaSeconds)))

(event Game|Damage|EventAnyDamage
  (params (Damage :type Float%20%28single-precision%29) (DamageType :type Damage%20Type%20Object%20Reference) (InstigatedBy :type Controller%20Object%20Reference) (DamageCauser :type Actor%20Object%20Reference))
  (bind _sparkp (Variables|Default|GetSparkP))
  (if (Variables|Default|GetbIsAlive)
    (Utilities|FlowControl|Sequence
      (:then_0
        (Variables|Default|SetHealth (- (Variables|Default|GetHealth) Damage)))
      (:then_1
        (bind _newvalue (CallFunction|ParticlePercentage 6.0))
        (Effects|Components|ParticleSystem|SetFloatParameter (Variables|Default|GetSmoke) "SpawnRate" _newvalue) ; 6
        (bind _newvalue_2 (CallFunction|ParticlePercentage 12.0))
        (Effects|Components|ParticleSystem|SetFloatParameter _sparkp "SpawnRateSpark" _newvalue_2) ; 12
        (bind _newvalue_3 (CallFunction|ParticlePercentage 2e+02))
        (Effects|Components|ParticleSystem|SetFloatParameter _sparkp "SpawnRateParticle" _newvalue_3) ; 100
      )
      (:then_2
        (if (<= (Variables|Default|GetHealth) 0.0)
          (Variables|Default|SetbIsAlive false)
          (Actor|Tick|SetActorTickEnabled false)
          (CallFunction|DeathRituals))))))

(event EventBeginPlay)

(fn ConstructionScript)

(fn ParticlePercentage
  (params (ParticleMaxRange :type Float%20%28single-precision%29))
  (bind _output_get (Variables|Default|SetHealthPercentLeft (* (/ (- 1e+02 (Variables|Default|GetHealth)) 1e+02) 1e+02)))
  (return (/ (* _output_get ParticleMaxRange) 1e+02)))

(fn HitEffects
  (params (Hit :type Hit%20Result%20Structure))
  (bind (_bblockinghit _binitialoverlap _time _distance _location _impactpoint _normal _impactnormal _physmat _hitactor _hitcomponent _hitbonename _hititem _faceindex _tracestart) (Collision|BreakHitResult Hit))
  (Class|HitEffectFunctionLibrary|PlayHitEffect Hit)
  (Utilities|IsValid _hitactor
    (:Is%20Valid
      (if (Variables|/Script/Engine.Actor|GetbCanBeDamaged _hitactor)
        (Game|Damage|ApplyPointDamage _hitactor 0.5 _tracestart Hit 0 self)))))

(fn IsDead
  (return (not (Variables|Default|GetbIsAlive))))