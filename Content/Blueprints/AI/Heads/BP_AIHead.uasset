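; BP_AIHead is a detached AI head actor that pops off as a physics prop when spawned.
; On BeginPlay it enables physics on the Head component and launches it upward with a randomized velocity-change impulse.
; It also plays a short-circuit particle effect and sound at its location, then creates a dynamic material on the second slot and zeroes its Health parameter.
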(event EventBeginPlay
  (bind _returnvalue (Transformation|GetActorLocation))
  (bind _head (Variables|Default|GetHead))
  (Physics|SetSimulatePhysics _head true)
  (Physics|AddImpulse _head (Math|Vector|MakeVector (Math|Random|RandomFloatinRange -1e+01 1e+01) (Math|Random|RandomFloatinRange -1e+01 1e+01) (Math|Random|RandomFloatinRange 3.5e+02 4.5e+02)) "None" true)
  (Effects|SpawnEmitteratLocation "/Game/Particles/P_ShotCircut.P_ShotCircut" _returnvalue "0, 0, 0" "0.500000,0.500000,0.500000")
  (Audio|SpawnSoundatLocation "/Game/Sounds/ShotCircut_Cue.ShotCircut_Cue" _returnvalue "0, 0, 0" 1.0 1.0 0.0 0 0)
  (bind _returnvalue_2 (Rendering|Material|CreateDynamicMaterialInstance (Variables|Default|GetHead) 1 0 "None" :!class /Script/Engine.PrimitiveComponent))
  (Utilities|IsValid _returnvalue_2
    (:Is%20Valid
      (Rendering|Material|SetScalarParameterValue _returnvalue_2 "Health" 0.0 :!class /Script/Engine.MaterialInstanceDynamic))))

(fn ConstructionScript)