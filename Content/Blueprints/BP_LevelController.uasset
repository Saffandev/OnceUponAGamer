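; BP_LevelController is a trigger-driven level streaming controller that loads and unloads configured sublevels when the PlayerCharacter overlaps its Trigger.
; The overlap calls Load/Unload, which asynchronously loads from LevelToLoad, making levels visible, and unloads from LevelToUnload.
; Each branch steps through its array by re-calling the event after each operation, resetting its index at the end.
; The Load flag is never read, so every call runs both branches.
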(event OnComponentBeginOverlap(Trigger)
  (params (OverlappedComponent :type Primitive%20Component%20Object%20Reference) (OtherActor :type Actor%20Object%20Reference) (OtherComp :type Primitive%20Component%20Object%20Reference) (OtherBodyIndex :type Integer) (bFromSweep :type Boolean) (SweepResult :type Hit%20Result%20Structure%20%28by%20ref%29))
  (Utilities|Casting|CastToPlayerCharacter OtherActor)
  (CallFunction|Load/Unload true))

(event Custom|Load/Unload
  (params (Load :type Boolean))
  (Utilities|FlowControl|Sequence
    (:then_0
      (if (not (== (Utilities|Array|Length (Variables|Default|GetLevelToLoad)) 0))
        (Class|GameplayStatics|LoadStreamLevelbySoftObjectPtr (Utilities|Array|Get(acopy) (Variables|Default|GetLevelToLoad) (Variables|Default|GetCurrentLevelLoadedNumber)) true false)
        (if (== (Utilities|Array|Length (Variables|Default|GetLevelToLoad)) (+ (Variables|Default|GetCurrentLevelLoadedNumber) 1))
          (Variables|Default|SetCurrentLevelLoadedNumber 0)
          (else
            (Math|Integer|IncrementInt (Variables|Default|GetCurrentLevelLoadedNumber)
              (:%20%20
                (CallFunction|Load/Unload true)))))))
    (:then_1
      (if (not (== (Utilities|Array|Length (Variables|Default|GetLevelToUnload)) 0))
        (Class|GameplayStatics|UnloadStreamLevelbySoftObjectPtr (Utilities|Array|Get(acopy) (Variables|Default|GetLevelToUnload) (Variables|Default|GetCurrentLevelUnloadedNumber)) false)
        (if (== (Utilities|Array|Length (Variables|Default|GetLevelToUnload)) (+ (Variables|Default|GetCurrentLevelUnloadedNumber) 1))
          (Variables|Default|SetCurrentLevelUnloadedNumber 0)
          (else
            (Math|Integer|IncrementInt (Variables|Default|GetCurrentLevelUnloadedNumber)
              (:%20%20
                (CallFunction|Load/Unload false)))))))))

(fn ConstructionScript)