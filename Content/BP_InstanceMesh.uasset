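; Construction-script actor that builds a row of Count copies of a chosen mesh with a hierarchical instanced static mesh component.
; Section Length calc sizes each step from the mesh bounds times the actor's X scale, used for all three axes.
; Adding Instance places copies along the selected axis, shifted by LocationOffset.
; The MeshTransform array, resized to Count + 1 with the last instance's transform in its final slot, then overwrites instance transforms by index.
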(event EventBeginPlay)

(event Collision|EventActorBeginOverlap
  (params (OtherActor :type Actor%20Object%20Reference)))

(event EventTick
  (params (DeltaSeconds :type Float%20%28single-precision%29)))

(fn ConstructionScript
  (bind _count (Variables|Default|Getcount))
  (Components|StaticMesh|SetStaticMesh (Variables|Default|GetHierarchicalInstancedStaticMesh) (Variables|Default|GetMesh))
  (|SectionLengthcalc)
  (Utilities|Array|Resize (Variables|Default|GetMeshTransform) (+ (Variables|Default|Getcount) 1))
  (for _index (range 1 (Variables|Default|Getcount))
    (Variables|Default|SetMeshIndex _index)
    (|AddingInstance))
  (Utilities|Array|SetArrayElem (Variables|Default|GetMeshTransform) _count (.OutInstanceTransform (Components|InstancedStaticMesh|GetInstanceTransform (Variables|Default|GetHierarchicalInstancedStaticMesh) (- _count 1) false)))
  (for (_array_element _array_index) (Variables|Default|GetMeshTransform)
    (Variables|Default|SetTransformIndex _array_index)
    (Components|InstancedStaticMesh|UpdateInstanceTransform (Variables|Default|GetHierarchicalInstancedStaticMesh) (Variables|Default|GetTransformIndex) _array_element false false false)))